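; Game instance Blueprint that creates the player HUD widget on Init and keeps its current-task display up to date.
; UpdateCurrentTaskWidget copies the TaskManagerSubsystem's current task title, description and item counts into the HUD's task widget, turning its outline green when the counts match.
; A separate function sets just the current item count, while UpdateTaskList is an empty stub.
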(event EventUpdateCurrentTaskWidget
  (params (Task :type Task%20Struct%20Structure))
  (CallFunction|UpdateCurrentTask (Variables|/Game/Blueprint/UI/PlayerHUd.PlayerHUD_C|GetCurrentTaskWidget (stale EventInit _output_get))))

(event EventInit
  (bind _returnvalue (UserInterface|CreateWidget "/Game/Blueprint/UI/PlayerHUd.PlayerHUD_C" (Game|GetPlayerController 0)))
  (bind _output_get (Variables|Default|SetPlayerHUD _returnvalue)))

(fn UpdateCurrentTask
  (params (TaskWidget :type Current%20Task%20Widget%20Object%20Reference))
  (bind _returnvalue (Class|TaskManagerSubsystem|GetCurrentTask (Subsystems|GetTaskManagerSubsystem)))
  (Rendering|Components|TextRender|SetText (Variables|/Game/Blueprint/UI/CurrentTaskWidget.CurrentTaskWidget_C|GetTaskTitle TaskWidget) (Utilities|Text|ToText(String) (.Title (Utilities|Struct|BreakTaskStruct _returnvalue))))
  (Rendering|Components|TextRender|SetText (Variables|/Game/Blueprint/UI/CurrentTaskWidget.CurrentTaskWidget_C|GetTaskDescription TaskWidget) (Utilities|Text|ToText(String) (.Description (Utilities|Struct|BreakTaskStruct _returnvalue))))
  (Rendering|Components|TextRender|SetText (Variables|/Game/Blueprint/UI/CurrentTaskWidget.CurrentTaskWidget_C|GetRequiredItemCount TaskWidget) (Utilities|Text|ToText(Integer) (.ItemRequirementCount (Utilities|Struct|BreakTaskStruct _returnvalue))))
  (Rendering|Components|TextRender|SetText (Variables|/Game/Blueprint/UI/CurrentTaskWidget.CurrentTaskWidget_C|GetCurrentItemCount TaskWidget) (Utilities|Text|ToText(Integer) (.CurrentItemCount (Utilities|Struct|BreakTaskStruct _returnvalue))))
  (if (== (.ItemRequirementCount (Utilities|Struct|BreakTaskStruct _returnvalue)) (.CurrentItemCount (Utilities|Struct|BreakTaskStruct _returnvalue)))
    (Class|Border|SetBrushColor (Variables|/Game/Blueprint/UI/CurrentTaskWidget.CurrentTaskWidget_C|GetOutline TaskWidget) (Class|KismetMathLibrary|LinearColorGreen))))

(fn UpdateTaskList
  (params (TaskListWidget :type Task%20List%20Widget%20Object%20Reference)))

(fn UpdateCurrentItemCount
  (params (TaskWidget :type Current%20Task%20Widget%20Object%20Reference%20%28by%20ref%29) (NewItemCount :type Integer))
  (Rendering|Components|TextRender|SetText (Variables|/Game/Blueprint/UI/CurrentTaskWidget.CurrentTaskWidget_C|GetCurrentItemCount TaskWidget) (Utilities|Text|ToText(Integer) NewItemCount)))